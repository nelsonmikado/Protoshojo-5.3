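; BP_Enemy1 is an enemy whose cube tracks the BP_ball along Y, much like an opposing paddle.
; Each Tick it looks up the ball, stores its sphere's relative location, and moves the cube toward that Y, clamped to fixed bounds, via MoveComponentTo.
; Any hit on the cube calls EnemyBlow on the ball.
; Health starts at HealthM and drops through TomaDeDaño, with no death handling here.
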(event OnComponentHit(Cube)
  (params (HitComponent :type Primitive%20Component%20Object%20Reference) (OtherActor :type Actor%20Object%20Reference) (OtherComp :type Primitive%20Component%20Object%20Reference) (NormalImpulse :type Vector :default "0, 0, 0") (Hit :type Hit%20Result%20Structure%20%28by%20ref%29))
  ;[1 1 1] On Hit
  (bind _returnvalue (Actor|GetActorOfClass "/Game/Main_Game/Blueprints/BP_ball.BP_ball_C"))
  (Default|EnemyBlow _returnvalue))

(event Custom|Cambio%20de%20Direccion
  ;[1 1 1] Movimiento
  (Components|MoveComponentTo (Variables|Default|GetCube) (Math|Vector|MakeVector 0.0 (Math|Float|Clamp(Float) (.y (Variables|Default|GetUbicación)) -475.0 475.0) 0.0) "0, 0, 0" false false (Variables|Default|GetOver%20Time) false))

(event EventBeginPlay
  ;[1 1 1] Health
  (Variables|Default|SetHealthE (Variables|Default|GetHealthM)))

(event EventTick
  (params (DeltaSeconds :type Float%20%28single-precision%29))
  ;[1 1 1] Movimiento
  (bind _returnvalue (Actor|GetActorOfClass "/Game/Main_Game/Blueprints/BP_ball.BP_ball_C"))
  (Utilities|IsValid _returnvalue
    (:Is%20Valid
      (Variables|Default|SetUbicación (Variables|/Script/Engine.SceneComponent|GetRelativeLocation (Variables|/Game/Main_Game/Blueprints/BP_ball.BP_ball_C|GetSphere _returnvalue)))
      (CallFunction|CambioDeDireccion))))

(event EventTomaDeDaño
  (params (Daño :type Float%20%28double-precision%29))
  ;[1 1 1] Health
  (Variables|Default|SetHealthE (- (Variables|Default|GetHealthE) Daño)))

(fn ConstructionScript)