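; BP_ball is a physics-driven ball actor that deals damage to actors it overlaps and can be hit in several ways.
; On BeginPlay it launches with a random impulse within X/Y ranges that the Force function can set.
; Shot up, shot down, enemy blow and straight blow functions apply further impulses, with the enemy blow randomized.
; Overlaps on Sphere1 send a fixed-damage message to the other actor, and a Destruction event destroys the ball.
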(event OnComponentBeginOverlap(Sphere1)
  (params (OverlappedComponent :type Primitive%20Component%20Object%20Reference) (OtherActor :type Actor%20Object%20Reference) (OtherComp :type Primitive%20Component%20Object%20Reference) (OtherBodyIndex :type Integer) (bFromSweep :type Boolean) (SweepResult :type Hit%20Result%20Structure%20%28by%20ref%29))
  (Class|BPIDaño|TomaDeDaño(Message) OtherActor 1e+01))

(event Custom|Destruction
  (CallFunction|BallDestroy))

(event EventBeginPlay
  (CallFunction|Initialforce))

(fn ConstructionScript)

(fn Force
  (params (MinX :type Float%20%28double-precision%29) (MinY :type Float%20%28double-precision%29) (MaxY :type Float%20%28double-precision%29) (MaxX :type Float%20%28double-precision%29))
  (Variables|Float|SetMinX MinX)
  (Variables|Float|SetMinY MinY)
  (Variables|Float|SetMaxY MaxY)
  (Variables|Float|SetMaxX MaxX))

(fn Initialforce
  (Physics|AddImpulse (Variables|Default|GetSphere) (Math|Vector|MakeVector (Math|Random|RandomFloatinRange (Variables|Float|GetMinX) (Variables|Float|GetMaxX)) (Math|Random|RandomFloatinRange (Variables|Float|GetMinY) (Variables|Float|GetMaxY)) (Variables|Float|GetImpulse%20Z)) "None" false))

(fn Shotup
  (Physics|AddImpulse (Variables|Default|GetSphere) (Math|Vector|MakeVector (Variables|Float|GetImpulse%20X) (Variables|Float|GetImpulse%20Y) (Variables|Float|GetImpulse%20Z)) "None" false))

(fn Shotdown
  (Physics|AddImpulse (Variables|Default|GetSphere) (Math|Vector|MakeVector (Variables|Float|GetImpulse%20X) (Variables|Float|GetImpulse%20-Y) (Variables|Float|GetImpulse%20Z)) "None" false))

(fn EnemyBlow
  (Physics|AddImpulse (Variables|Default|GetSphere) (Math|Vector|MakeVector (Math|Random|RandomFloatinRange (Variables|Float|GetBack%20Impulse%20X%20Min) (Variables|Float|GetBack%20Impulse%20X%20Max)) (Math|Random|RandomFloatinRange (Variables|Float|GetBack%20Impulse%20Y%20Min) (Variables|Float|GetBack%20Impulse%20Y%20Max)) (Variables|Float|GetBack%20Impulse%20Z)) "None" false))

(fn StraightBlow
  (Physics|AddImpulse (Variables|Default|GetSphere) (Math|Vector|MakeVector (Variables|Float|GetStraight) 0.0 0.0) "None" false))

(fn BallDestroy
  (Actor|DestroyActor))